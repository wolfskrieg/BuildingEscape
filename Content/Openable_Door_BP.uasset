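; Openable door actor that swings open and shut in response to events from its OpenDoor component.
; BeginPlay caches the initial rotation, and a timeline's OpenAngle track adds yaw to it to rotate the whole actor.
; OnOpen plays the timeline and OnClose reverses it, while an event track on the timeline plays the door lock sound at the actor's location.
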(event OnOpen(OpenDoor)
  (bind _openangle (Timeline|Timeline_0 Play)
    (:Update
      (Transformation|SetActorRotation (Math|Rotator|CombineRotators (Variables|Default|GetInitialRotation) (Math|Rotator|MakeRotator 0.0 0.0 (+ _openangle 0.0)))))
    (:SoundTiming
      (Audio|PlaySoundatLocation "/Game/Audio/door-lock.door-lock" (Transformation|GetActorLocation)))))

(event OnClose(OpenDoor)
  (bind _openangle (Timeline|Timeline_0 Reverse)
    (:Update
      (Transformation|SetActorRotation (Math|Rotator|CombineRotators (Variables|Default|GetInitialRotation) (Math|Rotator|MakeRotator 0.0 0.0 (+ _openangle 0.0)))))
    (:SoundTiming
      (Audio|PlaySoundatLocation "/Game/Audio/door-lock.door-lock" (Transformation|GetActorLocation)))))

(event EventBeginPlay
  (Variables|Default|SetInitialRotation (Transformation|GetActorRotation)))

(event Collision|EventActorBeginOverlap
  (params (OtherActor :type Actor%20Object%20Reference)))

(event EventTick
  (params (DeltaSeconds :type Float%20%28single-precision%29)))

(fn ConstructionScript)